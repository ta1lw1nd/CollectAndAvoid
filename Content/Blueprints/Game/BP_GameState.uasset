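; Game state that tracks the coin score and handles the win condition.
; On BeginPlay it sums the points of every BP_Coin in the level into TargetScore.
; AddScore raises the score, fires OnScoreChanged and prints both totals.
; Once the target is reached it updates GameStatus, pauses the game and shows WBP_Win with UI-only input and a visible cursor.
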(event `self.ReceiveBeginPlay`
  (bind _outactors (`GameplayStatics.GetAllActorsOfClass` "/Game/Blueprints/Coin/BP_Coin.BP_Coin_C"))
  (for _array_element _outactors
    (set `self.TargetScore` (+ (`/Game/Blueprints/Coin/BP_Coin.Points` _array_element) (`self.TargetScore`)))))

(fn `AddScore`
  (params (Points :type Integer))
  (bind _returnvalue (`GameplayStatics.GetPlayerController` 0))
  (bind _output_get (set `self.Score` (+ Points (`self.Score`))))
  (`self.OnScoreChanged` _output_get)
  (`KismetSystemLibrary.PrintString` (`KismetStringLibrary.Conv_IntToString` (`self.Score`)))
  (`KismetSystemLibrary.PrintString` (`KismetStringLibrary.Conv_IntToString` (`self.TargetScore`)))
  (if (>= _output_get (`self.TargetScore`))
    (set `self.GameStatus` "NewEnumerator1")
    (`GameplayStatics.SetGamePaused` true)
    (bind _returnvalue_2 (`|CreateWidget` "/Game/Blueprints/UI/WBP_Win.WBP_Win_C"))
    (`UserWidget.AddToViewport` _returnvalue_2 0)
    (`WidgetBlueprintLibrary.SetInputMode_UIOnlyEx` _returnvalue _returnvalue_2)
    (set `PlayerController.bShowMouseCursor` true _returnvalue)))

(fn `UserConstructionScript`)